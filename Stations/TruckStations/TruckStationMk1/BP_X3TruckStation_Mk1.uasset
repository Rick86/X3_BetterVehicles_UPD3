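; Blueprint for the X3 Mk1 truck station, a station variant that relies on its parent class for nearly all behavior.
; Its only working logic is ShowDropPoint, which shows or hides the DropPoint and Box components in game from a boolean.
; The construction script just calls the parent, and the event graph holds only disabled events and an unconnected unload-vehicle message call.
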(event EventBeginPlay
  (|CallParentFunction) ; This node is disabled and will not be called.\nDrag off pins to build functionality.
)

(event Collision|EventActorBeginOverlap
  (params (OtherActor :type Actor%20Object%20Reference))
  (|CallParentFunction OtherActor) ; This node is disabled and will not be called.\nDrag off pins to build functionality.
)

(event EventTick
  (params (DeltaSeconds :type Float%20%28single-precision%29))
  (|CallParentFunction DeltaSeconds) ; This node is disabled and will not be called.\nDrag off pins to build functionality.
)

(fn ConstructionScript
  (|CallParentFunction))

(fn ShowDropPoint
  (params (Show%20Drop-Point? :type Boolean))
  (bind _returnvalue (not Show%20Drop-Point?))
  (Development|SetHiddeninGame (Variables|Default|GetDropPoint) _returnvalue false)
  (Development|SetHiddeninGame (Variables|Default|GetBox) _returnvalue false))